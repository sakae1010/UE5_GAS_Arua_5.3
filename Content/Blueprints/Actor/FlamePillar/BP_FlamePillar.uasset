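; BP_FlamePillar is a flame pillar actor that gives its fire light a randomly varied, continuous flicker.
; From BeginPlay, it randomly picks one of two intensity timelines and plays it from the start.
; Each timeline update sets the FireLight intensity to the curve value times BaseIntensity.
; When a timeline finishes, it picks again, so the flicker loops without a fixed pattern.
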(event Custom|ChooseEvent_Event
  (switch int (Math|Random|RandomIntegerinRange 0 1)
    (:Default
      (CallFunction|TimeLineEvent2Event :!label _label))
    (:0
      (CallFunction|TimeLineEvent1Event))
    (:1
      (goto _label))))

(event Custom|TimeLineEvent_1_Event
  (bind _fireintensity (Timeline|FireIntensityTimeline_1 PlayFromStart)
    (:Update
      (CallFunction|UpdateFireIntensity _fireintensity))
    (:Finished
      (CallFunction|ChooseEventEvent))))

(event Custom|TimeLineEvent_2_Event
  (bind _fireintensity (Timeline|FireIntensityTimeline_2 PlayFromStart)
    (:Update
      (CallFunction|UpdateFireIntensity _fireintensity))
    (:Finished
      (CallFunction|ChooseEventEvent))))

(event EventBeginPlay
  (CallFunction|ChooseEventEvent))

(fn ConstructionScript)

(fn UpdateFireIntensity
  (params (Intensity :type Float%20%28double-precision%29))
  (Rendering|Components|Light|SetIntensity (Variables|Default|GetFireLight) (* Intensity (Variables|Default|GetBaseIntensity))))