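; Actor that fades its static mesh out and back in, running a one-second-delayed out-then-in cycle on BeginPlay.
; The construction script stores the original materials and builds dynamic instances from the fade materials.
; FadeOut applies these instances and plays a timeline driving their FadeValue parameter, while FadeIn reverses it.
; On finish, a negative value restores the materials and blocks the Visibility channel, while zero ignores that channel.
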(event Custom|FadeOut
  (CallFunction|SetMaterialsDynamicInstances)
  (bind _fadevalue (Timeline|FadeTimeline Play)
    (:Update
      (for _array_element (Variables|Default|GetDyamicMaterialInstances)
        (Rendering|Material|SetScalarParameterValue _array_element "FadeValue" _fadevalue :!class /Script/Engine.MaterialInstanceDynamic)))
    (:Finished
      (CallFunction|FadeFindished _fadevalue))))

(event Custom|FadeIn
  (bind _fadevalue (Timeline|FadeTimeline Reverse)
    (:Update
      (for _array_element (Variables|Default|GetDyamicMaterialInstances)
        (Rendering|Material|SetScalarParameterValue _array_element "FadeValue" _fadevalue :!class /Script/Engine.MaterialInstanceDynamic)))
    (:Finished
      (CallFunction|FadeFindished _fadevalue))))

(event EventBeginPlay
  (CallFunction|FadeOut)
  (Utilities|FlowControl|Delay 1.0)
  (CallFunction|Fadein))

(event Collision|EventActorBeginOverlap
  (params (OtherActor :type Actor%20Object%20Reference)))

(event EventTick
  (params (DeltaSeconds :type Float%20%28single-precision%29)))

(fn ConstructionScript
  (Utilities|Array|Clear (Variables|Default|GetDyamicMaterialInstances))
  (Variables|Default|SetOriginalMaterials (Rendering|Material|GetMaterials (Variables|Default|GetStaticMesh)))
  (for _array_element (Variables|Default|GetFadeMaterialInstances)
    (bind _returnvalue (Rendering|Material|CreateDynamicMaterialInstance _array_element "None" "None" :!class /Script/Engine.KismetMaterialLibrary))
    (Utilities|Array|AddUnique (Variables|Default|GetDyamicMaterialInstances) _returnvalue)))

(fn SetMaterialsDynamicInstances
  (for (_array_element _array_index) (Variables|Default|GetDyamicMaterialInstances)
    (Rendering|Material|SetMaterial (Variables|Default|GetStaticMesh) _array_index _array_element)))

(fn ResetMaterials
  (for (_array_element _array_index) (Variables|Default|GetOriginalMaterials)
    (Rendering|Material|SetMaterial (Variables|Default|GetStaticMesh) _array_index _array_element)))

(fn FadeFindished
  (params (InputPin :type Float%20%28single-precision%29))
  (if (> 0.0 InputPin)
    (CallFunction|ResetMaterials)
    (Collision|SetCollisionResponsetoChannel (Variables|Default|GetStaticMesh) "ECC_Visibility" "ECR_Block")
    (elif (<= InputPin 0.0)
      (Collision|SetCollisionResponsetoChannel (Variables|Default|GetStaticMesh) "ECC_Visibility" "ECR_Ignore"))))