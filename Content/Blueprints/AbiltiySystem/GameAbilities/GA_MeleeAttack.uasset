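; Melee attack Gameplay Ability that plays the goblin spear attack montage on an avatar implementing CombatInterface.
; On activation it passes the combat target's location to the avatar as a warp target, then plays the montage.
; A melee montage gameplay event triggers a debug sphere at the combat socket location; no damage is applied here.
; The ability ends when the montage completes, blends out, is interrupted or is cancelled.
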(event Ability|EventActivateAbility
  (bind _returnvalue (Ability|GetAvatarActorfromActorInfo))
  (bind _returnvalue_2 (Class|EnemyInterface|GetCombatTarget(Message) _returnvalue))
  (bind _ascombat_interface (Utilities|Casting|CastToCombatInterface _returnvalue))
  (Class|CombatInterface|UpdateWarpTarget _ascombat_interface (Transformation|GetActorLocation _returnvalue_2))
  (|PlayMontageandWaitProxy "None" "/Game/Assets/Enemies/Goblin/Animations/Spear/AM_Attack_GoblinSpear.AM_Attack_GoblinSpear" 1.0 "None" true 1.0 0.0 false
    (:then
      (Ability|Tasks|WaitGameplayEvent "(TagName=\"Event.Montage.Attack.Melee\")" 0
        (:EventReceived
          (bind _returnvalue_3 (Class|CombatInterface|GetCombatSocketLocation(Message) (Ability|GetAvatarActorfromActorInfo)))
          (Rendering|Debug|DrawDebugSphere _returnvalue_3 1e+01 8 "(R=1.000000,G=1.000000,B=1.000000,A=1.000000)" 3.0))))
    (:OnCompleted
      (Ability|EndAbility :!label _label))
    (:OnBlendOut
      (goto _label))
    (:OnInterrupted
      (goto _label))
    (:OnCancelled
      (goto _label))))

(event Ability|EventOnEndAbility
  (params (bWasCancelled :type Boolean)))