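; Arcane Shards gameplay ability that shows a magic circle, then lets the player pick a ground point for a series of radial-damage shards.
; On input press it spawns a point collection at the target, caches its ground points, updates the warp target and plays the cast montage.
; The montage event hides the circle and starts a looping timer, each tick damaging nearby players and firing a GameplayCue until all points are used.
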(event Custom|SpawnShard
  (if (< (Variables|Default|GetCount) (Variables|Default|GetNumPoints))
    (CallFunction|StoreShardSpawnLocation)
    (CallFunction|StorePlayerstoDamage)
    (for _array_element (Variables|Default|GetPlayersToDamage)
      (CallFunction|RadiaDamageTotPlayer _array_element))
    (Math|Integer|IncrementInt (Variables|Default|GetCount)
      (:%20%20
        (Class|GameplayAbility|ExecuteGameplayCuewithParams "(TagName=\"GameplayCue.ArcaneShards\")" (Ability|GameplayCue|MakeGameplayCueParameters :Location (Variables|Default|GetSpawnLocation)))))
    (else
      (Utilities|Time|ClearandInvalidateTimerbyHandle (Variables|Default|GetSapwnTimer))
      (Utilities|FlowControl|Delay 0.2)
      (Actor|DestroyActor (Variables|Default|GetPointCollection))
      (Ability|EndAbility))))

(event Ability|EventActivateAbility
  (Utilities|FlowControl|Sequence
    (:then_0
      ;[0.1612 0.6064 1] 顯示魔法陣
      (Class|PlayerInterface|ShowMagicCircle(Message) (Ability|GetAvatarActorfromActorInfo) 0))
    (:then_1
      (Ability|Tasks|WaitInputPress false
        (:OnPress
          ;[0.2155 0.8599 1] 取得滑鼠點擊位置
          (bind _datahandle (|TargetUnderMouse)
            (:ValidData
              (Variables|Default|SetMouseHitLocation (.ImpactPoint (Collision|BreakHitResult (Ability|TargetData|GetHitResultfromTargetData _datahandle))))
              (Utilities|FlowControl|Sequence
                (:then_0
                  ;[0.3728 0.4944 1] 建立 point collection
                  (bind _returnvalue (Game|SpawnActorfromClass "/Game/Blueprints/AbiltiySystem/Aura/Abilities/Arcane/ArcaneShards/BP_PointCollection.BP_PointCollection_C" (Math|Transform|MakeTransform (Variables|Default|GetMouseHitLocation) "0, 0, 0" "1.000000,1.000000,1.000000") "AlwaysSpawn" "MultiplyWithRoot" 0 0))
                  (bind _output_get (Variables|Default|SetPointCollection _returnvalue))
                  ;;[1 1 1] 快取是避免跑  loop get 每次都重新算一個坑
                  (Variables|Default|SetPoints (Class|PointCollection|GetGroundPoints _output_get (Variables|Default|GetSpawnLocation) (Variables|Default|GetNumPoints) (Math|Random|RandomFloatinRange 0.0 3.6e+02))))
                (:then_1
                  ;[1 0.6319 0.1795] Update Facing Target
                  (Class|CombatInterface|UpdateWarpTarget(Message) (Ability|GetAvatarActorfromActorInfo) (Variables|Default|GetMouseHitLocation)))
                (:then_2
                  ;[1 0 0.09186] 播放 Montage and wait for Event
                  (|PlayMontageandWaitProxy "None" "/Game/Assets/Characters/Aura/Animations/Abilities/AM_Cast_ArcaneShards.AM_Cast_ArcaneShards" 1.0 "None" false 1.0 0.0 false
                    (:then
                      (Ability|Tasks|WaitGameplayEvent "(TagName=\"Event.Montage.ArcaneShards\")" 0 true
                        (:EventReceived
                          ;[1 1 1] 註冊時間 啟動時啟動一個
                          (bind _returnvalue_2 (Utilities|Time|SetTimerbyEvent (delegate Custom|SpawnShard) (Variables|Default|GetShardSwpanDeltaTime) true))
                          (Variables|Default|SetSapwnTimer _returnvalue_2)
                          (Class|PlayerInterface|HideMagicCircle(Message) (Ability|GetAvatarActorfromActorInfo))
                          (CallFunction|SpawnShard))))))))))))))

(event Ability|EventOnEndAbility
  (params (bWasCancelled :type Boolean)))

(fn StoreShardSpawnLocation
  (Variables|Default|SetSpawnLocation (Transformation|GetWorldLocation (Utilities|Array|Get(acopy) (Variables|Default|GetPoints) (Variables|Default|GetCount)))))

(fn StorePlayerstoDamage
  (bind _returnvalue (Ability|GetAvatarActorfromActorInfo))
  (bind _outoverlappingactors (Class|AuraAbilitySystemLibrary|GetLivePlayerWithinRadius _returnvalue (Utilities|Array|MakeArray _returnvalue) (Variables|Default|GetRadialDamageOuterRadius) (Variables|Default|GetSpawnLocation)))
  (Variables|Default|SetPlayersToDamage _outoverlappingactors))

(fn RadiaDamageTotPlayer
  (params (TargetActor :type Actor%20Object%20Reference))
  (Class|AuraAbilitySystemLibrary|ApplyDamageEffectParams (Class|AuraDamageGameplayAbility|MakeDamageEffectParams TargetActor (Variables|Default|GetSpawnLocation))))