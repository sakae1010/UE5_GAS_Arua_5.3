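; Passive startup gameplay ability for Aura that turns incoming Attributes gameplay events into attribute-driven effects on its owner.
; On activation it waits for events under the Attributes tag hierarchy, then builds a spec from EventBasedEffectClass.
; It loops over EventTags, setting the exactly matching tag's SetByCaller magnitude to the event magnitude and all others to zero.
; The finished spec is applied to self, and the graph never ends the ability.
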(event Ability|EventActivateAbility
  (bind _returnvalue (Ability|GetAbilitySystemComponentfromActorInfo))
  (bind _payload (Ability|Tasks|WaitGameplayEvent "(TagName=\"Attributes\")" 0 false false)
    (:EventReceived
      (Variables|Default|SetEventTag (.EventTag (Utilities|Struct|BreakGameplayEventData _payload)))
      (Variables|Default|SetEventMagnitude (.EventMagnitude (Utilities|Struct|BreakGameplayEventData _payload)))
      (Variables|Default|SetEventSpec (GameplayEffects|MakeOutgoingSpec _returnvalue (Variables|Default|GetEventBasedEffectClass) 1.0 (GameplayEffects|MakeEffectContext _returnvalue)))
      (for _array_element (Variables|Default|GetEventTags)
        (if (GameplayTags|MatchesTag _array_element (Variables|Default|GetEventTag) true)
          (Ability|GameplayEffect|AssignTagSetbyCallerMagnitude (Variables|Default|GetEventSpec) (Variables|Default|GetEventTag) (Variables|Default|GetEventMagnitude))
          (else
            (Ability|GameplayEffect|AssignTagSetbyCallerMagnitude (Variables|Default|GetEventSpec) _array_element 0.0))))
      (GameplayEffects|ApplyGameplayEffectSpecToSelf (Ability|GetAbilitySystemComponentfromActorInfo) (Variables|Default|GetEventSpec)))))

(event Ability|EventOnEndAbility
  (params (bWasCancelled :type Boolean)))