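; Gameplay ability for the Fire Bolt spell, which fires homing projectiles at the target under the mouse.
; It commits cost and cooldown, takes the hit location and actor from cursor target data, and updates the avatar's warp target.
; The cast montage's gameplay event triggers the spawn from the weapon socket with an overridden upward pitch, homing on the hit actor.
; The ability ends when the montage completes, blends out, is interrupted or is cancelled.
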(event Ability|EventActivateAbility
  ;[1 1 1] Cost And CD 都會檢查
  (Ability|CommitAbility)
  (bind _datahandle (|TargetUnderMouse)
    (:ValidData
      (Variables|Default|SetTargetLocation (.Location (Collision|BreakHitResult (Ability|TargetData|GetHitResultfromTargetData _datahandle))))
      (Variables|Default|SetMouseActor (.HitActor (Collision|BreakHitResult (Ability|TargetData|GetHitResultfromTargetData _datahandle))))
      (Class|CombatInterface|UpdateWarpTarget(Message) (Ability|GetAvatarActorfromActorInfo) (Variables|Default|GetTargetLocation))
      (|PlayMontageandWaitProxy "None" "/Game/Assets/Characters/Aura/Animations/Abilities/AM_Cast_FireBolt.AM_Cast_FireBolt" 1.0 "None" false 1.0 0.0 false
        (:then
          (Ability|Tasks|WaitGameplayEvent "(TagName=\"Event.Montage.FireBolt\")" 0
            (:EventReceived
              (Class|AuraFireBolt|SawnProjectiles (Variables|Default|GetTargetLocation) (GameplayTags|MakeLiteralGameplayTag "(TagName=\"CombatSocket.Weapon\")") true 45.0 (Variables|Default|GetMouseActor)))))
        (:OnCompleted
          (Ability|EndAbility :!label _label))
        (:OnBlendOut
          (goto _label))
        (:OnInterrupted
          (goto _label))
        (:OnCancelled
          (goto _label))))))

(event Ability|EventOnEndAbility
  (params (bWasCancelled :type Boolean)))