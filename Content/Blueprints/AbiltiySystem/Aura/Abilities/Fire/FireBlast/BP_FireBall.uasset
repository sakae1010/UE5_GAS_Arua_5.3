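; BP_FireBall is the Fire Blast ability's projectile, which flies outward, returns to ReturnActor and explodes near it.
; On authority, chained timelines lerp it to a forward apex, then back toward the actor's current location.
; Within explode distance it calls OnHit, applies radial damage to nearby live players except its owner, then destroys itself.
; Each target gets knockback away from the blast at a fixed upward pitch, plus a death impulse.
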(event EventBeginPlay)

(event Collision|EventActorBeginOverlap
  (params (OtherActor :type Actor%20Object%20Reference)))

(event EventTick
  (params (DeltaSeconds :type Float%20%28single-precision%29)))

(event EventStartOutgoingTimeline
  (bind _returnvalue (Components|GetOwner))
  (bind _array (Utilities|Array|MakeArray _returnvalue))
  (Networking|SwitchHasAuthority
    (:Authority
      ;[1 0.5411 0.1046] 收集 初始位置以及前進位置
      (Variables|Default|SetInitLocation (Transformation|GetActorLocation))
      (Variables|Default|SetApexLocation (+ (Variables|Default|GetInitLocation) (* (Transformation|GetActorForwardVector) (Variables|Default|GetTravelDistatance))))
      (bind _outgoingtrack (Timeline|OutgoingTimeline Play)
        (:Update
          (Transformation|SetActorLocation (Math|Vector|Lerp(Vector) (Variables|Default|GetInitLocation) (Variables|Default|GetApexLocation) _outgoingtrack) false false))
        (:Finished
          (bind _returntrack (Timeline|ReturningTimeline Play)
            (:Update
              (Transformation|SetActorLocation (Math|Vector|Lerp(Vector) (Variables|Default|GetApexLocation) (Transformation|GetActorLocation (Variables|Default|GetReturnActor)) _returntrack) false false)
              (if (CallFunction|IsWithinExplodeDistance)
                (Class|AuraProjectile|OnHit)
                (Utilities|Array|Add _array self)
                (bind _outoverlappingactors (Class|AuraAbilitySystemLibrary|GetLivePlayerWithinRadius self _array (Variables|Default|GetRadialDamageOuterRadius) (Transformation|GetActorLocation)))
                (Class|AuraAbilitySystemLibrary|SetIsRadialDamageEffectParams (Variables|Default|GetExplosionDamageParams) true (Variables|Default|GetRadialDamageInnerRadius) (Variables|Default|GetRadialDamageOuterRadius) (Transformation|GetActorLocation))
                (for _array_element _outoverlappingactors
                  (Class|AuraAbilitySystemLibrary|SetEffectParmsTargetASC (Variables|Default|GetExplosionDamageParams) (Ability|GetAbilitySystemComponent _array_element))
                  (Variables|Default|SetKnockbackDirection (- (Transformation|GetActorLocation _array_element) (Transformation|GetActorLocation)))
                  (Class|AuraAbilitySystemLibrary|SetKnockbackDirection (Variables|Default|GetExplosionDamageParams) (CallFunction|OverrideKnockbackPitch) (Variables|Default|GetKnockbackMagnitude))
                  (Class|AuraAbilitySystemLibrary|SetDeathImpulseDirection (Variables|Default|GetExplosionDamageParams) (Variables|Default|GetKnockbackDirection) (Variables|Default|GetDeathimpulseMagnitude))
                  (Class|AuraAbilitySystemLibrary|ApplyDamageEffectParams (Variables|Default|GetExplosionDamageParams)))
                (Actor|DestroyActor)))))))))

(fn ConstructionScript)

(fn IsWithinExplodeDistance
  (return (<= (Math|Vector|VectorLength (- (Transformation|GetActorLocation) (Transformation|GetActorLocation (Variables|Default|GetReturnActor)))) (Variables|Default|GetExplodeDistance))))

(fn OverrideKnockbackPitch
  (bind _knockbackdirection (Variables|Default|GetKnockbackDirection))
  (bind _returnvalue (Math|Rotator|MakeRotfromX _knockbackdirection))
  (return (Math|Vector|GetForwardVector (Math|Rotator|MakeRotator (.roll _returnvalue) 45.0 (.yaw _returnvalue)))))